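; Behavior tree task that moves the AI controller's pawn to the third TargetPoint found in the level or to its mirrored position.
; A FlipFlop alternates between the point's location and that vector yawed 180 degrees around world origin.
; The mirrored branch loops back after a short delay into the direct move, which waits, then finishes as failed.
; The Enemy3 lookup feeds only unconnected stop-movement and arrival-check nodes.
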(event `self.ReceiveExecuteAI`
  (params (OwnerController :type "AIController Object Reference") (ControlledPawn :type "Pawn Object Reference"))
  (bind _returnvalue (`GameplayStatics.GetActorOfClass` "/Game/Enemies/Enemy3.Enemy3_C"))
  (`/Engine/EditorBlueprintResources/StandardMacros.FlipFlop` :!label _label
    (:`A`
      (bind _outactors (`GameplayStatics.GetAllActorsOfClass` "/Script/Engine.TargetPoint"))
      (`AIBlueprintHelperLibrary.SimpleMoveToLocation` OwnerController (`Actor.K2_GetActorLocation` (`|GetArrayItem` _outactors 2)))
      (`KismetSystemLibrary.Delay` 1.0)
      (`self.FinishExecute` false))
    (:`B`
      (bind _outactors_2 (`GameplayStatics.GetAllActorsOfClass` "/Script/Engine.TargetPoint"))
      (`AIBlueprintHelperLibrary.SimpleMoveToLocation` OwnerController (`KismetMathLibrary.GreaterGreater_VectorRotator` (`Actor.K2_GetActorLocation` (`|GetArrayItem` _outactors_2 2)) (struct :`Pitch` 180.0)))
      (`KismetSystemLibrary.Delay` 0.5)
      (goto _label))))